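; HitBox is a melee hit check that runs once on BeginPlay and damages what it hits.
; It gets the owning player's HappieCharacterBP and box-traces for Pawns between its left lower-arm and hand sockets, with debug drawing.
; The hit actor takes fixed damage, credited to the owning controller, unless it equals the opposite PlayerController (a controller-to-actor comparison, not a pawn check).
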(event EventBeginPlay
  (bind _ashappie_character_bp (Utilities|Casting|CastToHappieCharacterBP (Game|Player|GetPlayerPawn (Variables|Default|GetOwningPlayerIndex))))
  (bind _outhit (Class|KismetSystemLibrary|BoxTraceSingleforObjects (Transformation|GetSocketLocation (Variables|/Script/Engine.Character|GetMesh _ashappie_character_bp) "lowerarm_lSocket") (Transformation|GetSocketLocation (Variables|/Script/Engine.Character|GetMesh _ashappie_character_bp) "hand_lSocket") "2.000000,14.000000,14.000000" "0, 0, 0" (Utilities|Array|MakeArray "ObjectTypeQuery3") false 0 "ForDuration" true))
  (if (not (== (Game|GetPlayerController (Variables|Default|GetOppositeControllerIndex)) (.hitactor _outhit)))
    (Game|Damage|ApplyDamage (.hitactor _outhit) 5.0 (Game|GetPlayerController (Variables|Default|GetOwningPlayerIndex)) _ashappie_character_bp)))

(fn ConstructionScript)